(event Custom|Attaquer
  (bind _returnvalue (Game|GetPlayerCharacter 0))
  (bind _charactermovement (Variables|/Script/Engine.Character|GetCharacterMovement _returnvalue))
  ;[1 1 1] Animation corps à corps si arme
  (switch Utilities|FlowControl|Switch|SwitchonEnum_ArmeType (Variables|/Game/Blueprints/Objects/TYPES/BP_Object_Arme.BP_Object_Arme_C|GettypeArme (stale Input|ActionEvents|InputActionUtiliser _asbp_object_arme))
    (:NewEnumerator0
      (Variables|Weapons|SetisNormalAttack false))
    (:NewEnumerator1
      (Variables|Weapons|SetisHacheAttack false)))
  (Pawn|Components|CharacterMovement|SetMovementMode _charactermovement "MOVE_Walking" 0)
  (Utilities|FlowControl|Delay 0.2)
  (Utilities|FlowControl|DoOnce false) ; enters at Reset
)

(event Custom|ConstruireObject
  (bind _returnvalue (Transformation|GetActorLocation))
  ;[1 1 1] Construire l'object en l'alignant sur la grille du landscape
  (bind _outhit (Collision|LineTraceByChannel _returnvalue (+ (* (Math|Vector|GetForwardVector (Variables|MyCharacter|GetFollowCamera)) 5e+02) _returnvalue) "TraceTypeQuery1" false 0 "None"))
  (if (== (Utilities|GetClass (.HitActor (Collision|BreakHitResult _outhit))) "/Script/Landscape.Landscape")
    (Transformation|SetActorLocation (Variables|Construction|GetobjectConstruction) (Class|KismetMathLibrary|VectorSnappedtoGrid (.Location (Collision|BreakHitResult _outhit)) (Variables|Construction|GetsizeGridConstruction)) false false)))

(event EventBeginPlay
  ;[1 1 1] Créer la fenêtre principale + barre d'actions
  (Default|CreateMainUI (CallFunction|CastPlayerControllerCustom)))

(event EventTick
  (params (DeltaSeconds :type Float%20%28single-precision%29))
  ;[1 1 1] Vérifie que l'on peut CRAFT
  (if (Variables|Construction|GetisConstruction)
    (CallFunction|ConstruireObject)))

(event Input|ActionEvents|InputActionInteraction
  (params (Key :type Key%20Structure :default "None"))
  ;[1 1 1] Interagir object
  (:Pressed
    (RamasserObject|HitActorMethod)))

(event Input|ActionEvents|InputActionSprint
  (params (Key :type Key%20Structure :default "None"))
  (bind _charactermovement (Variables|Character|GetCharacterMovement))
  ;[1 1 1] Gestion du Sprint
  (:Pressed
    (Variables|/Script/Engine.CharacterMovementComponent|SetMaxWalkSpeed _charactermovement 5e+02))
  (:Released
    (Variables|/Script/Engine.CharacterMovementComponent|SetMaxWalkSpeed _charactermovement 1.5e+02)))

(event Input|ActionEvents|InputActionSeBaisser
  (params (Key :type Key%20Structure :default "None"))
  ;[1 1 1] Gestion du fait de ce baisser
  (:Pressed
    (Character|Crouch))
  (:Released
    (Character|UnCrouch)))

(event Input|ActionEvents|InputActionUtiliser
  (params (Key :type Key%20Structure :default "None"))
  (:Pressed
    (Utilities|FlowControl|Sequence
      (:then_0
        (if (and (Variables|Weapons|GethasCac) (not (Variables|Construction|GetisConstruction)))
          ;[1 1 1] Animation corps à corps si arme
          (Utilities|FlowControl|DoOnce false
            (:Completed
              (if (and (not (Variables|Weapons|GetisNormalAttack)) (Variables|Weapons|GethasCac))
                (bind _asbp_object_arme (Utilities|Casting|CastToBP_Object_Arme (Variables|Objects|GetobjectEquipe)))
                (switch Utilities|FlowControl|Switch|SwitchonEnum_ArmeType (Variables|/Game/Blueprints/Objects/TYPES/BP_Object_Arme.BP_Object_Arme_C|GettypeArme _asbp_object_arme)
                  (:NewEnumerator0
                    (Variables|Weapons|SetisNormalAttack true))
                  (:NewEnumerator1
                    (Variables|Weapons|SetisHacheAttack true)))
                (Pawn|Components|CharacterMovement|DisableMovement (Variables|/Script/Engine.Character|GetCharacterMovement (Game|GetPlayerCharacter 0)))
                (Utilities|Time|SetTimerbyEvent (delegate Custom|Attaquer) 1.0)
                (Armes(General)|HitActorClick))))))
      (:then_1
        (if (Variables|Construction|GetisConstruction)
          (DeposerObject|ValideDeposerObject))))))

(event Input|AxisEvents|InputAxisLookUp
  (params (AxisValue :type Float%20%28single-precision%29))
  ;[1 1 1] Caméra
  (Pawn|Input|AddControllerPitchInput AxisValue))

(event Input|AxisEvents|InputAxisTurn
  (params (AxisValue :type Float%20%28single-precision%29))
  ;[1 1 1] Caméra
  (Pawn|Input|AddControllerYawInput AxisValue))

(event Input|AxisEvents|InputAxisMoveForward
  (params (AxisValue :type Float%20%28single-precision%29))
  ;[1 1 1] Se déplacer
  (Pawn|Input|AddMovementInput (Math|Vector|GetForwardVector (Math|Rotator|MakeRotator 0.0 0.0 (.Yaw (Math|Rotator|BreakRotator (Pawn|GetControlRotation :!class /Script/Engine.Pawn))))) AxisValue false))

(event Input|AxisEvents|InputAxisMoveRight
  (params (AxisValue :type Float%20%28single-precision%29))
  ;[1 1 1] Se déplacer
  (Pawn|Input|AddMovementInput (Math|Vector|GetRightVector (Math|Rotator|MakeRotator 0.0 0.0 (.Yaw (Math|Rotator|BreakRotator (Pawn|GetControlRotation :!class /Script/Engine.Pawn))))) AxisValue false))

(event Input|KeyboardEvents|Tab
  (params (Key :type Key%20Structure :default "None"))
  (bind _asplayer_controller_custom (CallFunction|CastPlayerControllerCustom))
  ;[1 1 1] Ouvrir inventaire
  (:Pressed
    (Utilities|FlowControl|FlipFlop
      (:A
        (Default|OpenInventaire _asplayer_controller_custom))
      (:B
        (Default|CloseInventaire _asplayer_controller_custom)))))

(fn ConstructionScript)

(fn SpawnColis
  (params (actorToSpawn :type BP%20Object%20Class%20Reference))
  (Variables|Objects|SetspawnedItem actorToSpawn)
  (Variables|Move|SetjeterEnCours true)
  (Utilities|Time|SetTimerbyFunctionName self "resetTimerJeterObject" 0.3))

(fn HitActorMethod
  (bind (_start _end) (|Coordinates))
  (bind _outhit (Collision|SphereTraceByChannel _start _end 6e+01 "TraceTypeQuery1" false 0 "None"))
  (bind _output_get (Variables|Objects|SethitActorRamasser (.HitActor (Collision|BreakHitResult _outhit))))
  (if (and (Utilities|IsValid _output_get) (Utilities|DoesObjectImplementInterface _output_get "/Game/System/BP_Interface.BP_Interface_C"))
    (Variables|Move|SetramasserEnCours true)
    (Utilities|Time|SetTimerbyFunctionName self "resetTimerRamasserObject" 0.3)))

(fn GestionVie
  (params (value :type Float%20%28single-precision%29))
  (bind _structout (Utilities|Struct|SetmembersinStruct_HeroConstantes (Variables|Constantes|Getconstantes) (Math|Float|Clamp(Float) (+ (.vie (Utilities|Struct|BreakStruct_HeroConstantes (Variables|Constantes|Getconstantes))) value) 0.0 (.vieMax (Utilities|Struct|BreakStruct_HeroConstantes (Variables|Constantes|Getconstantes))))))
  (Variables|Constantes|Setconstantes _structout))

(fn ResetTimerJeterObject
  (bind _returnvalue (Game|GetPlayerCharacter 0))
  (bind _returnvalue_2 (Transformation|GetActorLocation _returnvalue))
  (Variables|Move|SetjeterEnCours false)
  ;[1 1 1] Fait Spawn l'objet
  (bind _returnvalue_3 (Game|SpawnActorfromClass "/Game/Blueprints/Objects/Colis/BP_Colis.BP_Colis_C" (Math|Transform|MakeTransform (+ (Math|Vector|MakeVector (.x _returnvalue_2) (.y _returnvalue_2) (* (.z _returnvalue_2) 0.6)) (* (Transformation|GetActorForwardVector _returnvalue) 100)) "0, 0, 0" "0.800000,0.800000,0.800000") "AdjustIfPossibleButAlwaysSpawn" 0 (Variables|Objects|GetspawnedItem) (Utilities|GetClassDefaults (Variables|Objects|GetspawnedItem)) 0))
  ;[1 1 1] Ajoute une durée de vie à l'objet
  (bind _output_get (LocalVariables|SetSpawnColis _returnvalue_3))
  (Actor|SetLifeSpan _output_get 15.0)
  ;[1 1 1] Active la physique et ajoute une force
  (Physics|SetSimulatePhysics (Variables|/Game/Blueprints/Objects/BP_Object.BP_Object_C|GetMesh (LocalVariables|GetSpawnColis)) true)
  (Physics|AddImpulse (Variables|/Game/Blueprints/Objects/BP_Object.BP_Object_C|GetMesh (LocalVariables|GetSpawnColis)) (* (Transformation|GetActorForwardVector (Game|GetPlayerCharacter 0)) 2000) "None" false))

(fn ResetTimerRamasserObject
  (Variables|Move|SetramasserEnCours false)
  ;[1 1 1] Si on ramasse un colis
  (bind _asbp_colis (Utilities|Casting|CastToBP_Colis (Variables|Objects|GethitActorRamasser))
    (:then
      (Default|IInteractionColis _asbp_colis (Variables|/Game/Blueprints/Objects/Colis/BP_Colis.BP_Colis_C|GetclassInColis _asbp_colis)))
    (:CastFailed
      ;[1 1 1] Si on ramsse un object qui n'est pas un colis
      (Class|BPInterface|IInteraction(Message) (Variables|Objects|GethitActorRamasser)))))

(fn EquiperCac
  (params (armeToEquip :type BP%20Object%20Class%20Reference))
  (bind _structure (Utilities|GetClassDefaults armeToEquip))
  (bind _mesh (Variables|Character|GetMesh))
  (Armes(General)|ResetArmes)
  ;[1 1 1] Si on a deja une arme equipee, on la supprime
  (Utilities|IsValid (Variables|Objects|GetobjectEquipe)
    (:Is%20Valid
      (Transformation|DetachFromComponent (Variables|/Script/Engine.Actor|GetRootComponent (Variables|Objects|GetobjectEquipe)) "KeepRelative" "KeepRelative" "KeepRelative" true)
      (Actor|DestroyActor (Variables|Objects|GetobjectEquipe)))
    (:Is%20Not%20Valid
      _))
  ;[1 1 1] Spawn l'arme en jeu
  (bind _returnvalue (Game|SpawnActorfromClass armeToEquip (Transformation|GetSocketTransform _mesh (Class|SkinnedMeshComponent|GetSocketBoneName _mesh "cac_socket") "RTS_World") "AlwaysSpawn" 0 _structure 0))
  ;[1 1 1] Message informant l'arme équipée
  (CallFunction|PrintStringInformation (Utilities|Text|ToText(String) (Utilities|String|Append (Utilities|String|ToString(Name) (Utilities|Struct|BreakStruct_Object _structure)) " équipé(e)")) true 2.0)
  (bind _output_get (Variables|Objects|SetobjectEquipe _returnvalue))
  (Collision|SetActorEnableCollision _returnvalue false)
  ;[1 1 1] Attache l'arme sur le personnage
  (Transformation|AttachComponentToComponent (Variables|Objects|GetobjectEquipe) (Variables|Character|GetMesh) "cac_socket" "SnapToTarget" "SnapToTarget" "SnapToTarget" true)
  (Rendering|SetVisibility (Variables|/Script/Engine.Actor|GetRootComponent (Variables|Objects|GetobjectEquipe)) false false)
  (Variables|Weapons|SetisArmedCac true)
  (Utilities|Time|SetTimerbyFunctionName 0 "resetTimerEquiperCac" 0.4)
  ;[1 1 1] Ferme l'inventaire
  (Default|CloseInventaire (CallFunction|CastPlayerControllerCustom)))

(fn ResetTimerEquiperCac
  (Rendering|SetVisibility (Variables|/Script/Engine.Actor|GetRootComponent (Variables|Objects|GetobjectEquipe)) true false)
  (Audio|PlaySound2D "/Game/Sounds/Cue_Equiper_Stuff.Cue_Equiper_Stuff" 1.0 1.0 0.0 0 0)
  (Variables|Weapons|SetisArmedCac false)
  (Variables|Weapons|SethasCac true))

(fn EquipeDistance
  (params (armeToEquipe :type BP%20Object%20Class%20Reference))
  (bind _structure (Utilities|GetClassDefaults armeToEquipe))
  (Armes(General)|ResetArmes)
  ;[1 1 1] Si on a deja une arme equipee, on la supprime
  (Utilities|IsValid (Variables|Objects|GetobjectEquipe)
    (:Is%20Valid
      (Transformation|DetachFromComponent (Variables|/Script/Engine.Actor|GetRootComponent (Variables|Objects|GetobjectEquipe)) "KeepRelative" "KeepRelative" "KeepRelative" true)
      (Actor|DestroyActor (Variables|Objects|GetobjectEquipe)))
    (:Is%20Not%20Valid
      _))
  ;[1 1 1] Spawn l'arme sur le jeu
  (bind _returnvalue (Game|SpawnActorfromClass armeToEquipe (Math|Transform|MakeTransform "0, 0, 0" "0, 0, 0" "1,1,1") "AlwaysSpawn" 0 _structure 0))
  (bind _output_get (Variables|Objects|SetobjectEquipe _returnvalue))
  ;[1 1 1] Message informant l'arme équipée
  (CallFunction|PrintStringInformation (Utilities|Text|ToText(String) (Utilities|String|Append (Utilities|String|ToString(Name) (Utilities|Struct|BreakStruct_Object _structure)) " équipé(e)")) true 2.0)
  (Collision|SetActorEnableCollision _output_get false)
  ;[1 1 1] Attache l'arme au personnage
  (Transformation|AttachComponentToComponent (Variables|Objects|GetobjectEquipe) (Variables|Character|GetMesh) "distance_socket" "SnapToTarget" "SnapToTarget" "SnapToTarget" true)
  (Rendering|SetVisibility (Variables|/Script/Engine.Actor|GetRootComponent (Variables|Objects|GetobjectEquipe)) false false)
  (Variables|Distance|SetisArmedDistance true)
  (Utilities|Time|SetTimerbyFunctionName 0 "resetTimerEquiperGun" 0.4)
  ;[1 1 1] Ferme l'inventaire
  (Default|CloseInventaire (CallFunction|CastPlayerControllerCustom)))

(fn ResetTimerEquiperGun
  (Rendering|SetVisibility (Variables|/Script/Engine.Actor|GetRootComponent (Variables|Objects|GetobjectEquipe)) true false)
  (Audio|PlaySound2D "/Game/Sounds/Cue_Equiper_Stuff.Cue_Equiper_Stuff" 1.0 1.0 0.0 0 0)
  (Variables|Distance|SetisArmedDistance false)
  (Variables|Distance|SethasDistance true))

(fn ResetArmes
  (Utilities|FlowControl|Sequence
    (:then_0
      (Variables|Weapons|SetisArmedCac false))
    (:then_1
      (Variables|Weapons|SethasCac false))
    (:then_2
      (Variables|Distance|SetisArmedDistance false))
    (:then_3
      (Variables|Distance|SethasDistance false))))

(fn HitActorClick
  (bind _followcamera (Variables|MyCharacter|GetFollowCamera))
  (bind _returnvalue (Transformation|GetWorldLocation _followcamera))
  (bind _returnvalue_2 (Math|Vector|GetForwardVector _followcamera))
  (bind _outhit (Collision|SphereTraceByChannel (+ _returnvalue (* _returnvalue_2 (Math|Float|Truncate (Variables|/Script/Engine.SpringArmComponent|GetTargetArmLength (Variables|MyCharacter|GetCameraBoom))))) (+ _returnvalue (* _returnvalue_2 400)) 6e+01 "TraceTypeQuery1" false 0 "None"))
  (Utilities|IsValid (.HitActor (Collision|BreakHitResult _outhit))
    (:Is%20Valid
      (bind _asbp_arbre (Utilities|Casting|CastToBP_Arbre (.HitActor (Collision|BreakHitResult _outhit))))
      (LocalVariables|SetarbreHit _asbp_arbre)
      (bind _asbp_object_arme (Utilities|Casting|CastToBP_Object_Arme (Variables|Objects|GetobjectEquipe)))
      (switch Utilities|FlowControl|Switch|SwitchonEnum_ArmeType (Variables|/Game/Blueprints/Objects/TYPES/BP_Object_Arme.BP_Object_Arme_C|GettypeArme _asbp_object_arme)
        (:NewEnumerator0
          (Nature|AbimerObject (LocalVariables|GetarbreHit) -5.0))
        (:NewEnumerator1
          (Nature|AbimerObject (LocalVariables|GetarbreHit) -25.0))))))

(fn AbimerObject
  (params (objectAbimer :type BP%20Arbre%20Object%20Reference) (damages :type Float%20%28single-precision%29))
  ;[1 1 1] Retirer vie à l'arbre
  (Default|GestionVie objectAbimer damages))

(fn DeposerObjectCraft
  (params (object :type BP%20Object%20Class%20Reference))
  ;[1 1 1] Faire spawn l'object pour le déposer au sol
  (bind _returnvalue (Game|SpawnActorfromClass object (Math|Transform|MakeTransform "0, 0, 0" "0, 0, 0" "1,1,1") "Undefined" 0 (Utilities|GetClassDefaults object) 0))
  (bind _output_get (Variables|Construction|SetobjectConstruction _returnvalue))
  (Collision|SetActorEnableCollision _output_get false)
  (Variables|Construction|SetisConstruction true)
  (Default|CloseInventaire (CallFunction|CastPlayerControllerCustom)))

(fn ValideDeposerObject
  (CallFunction|PrintStringInformation (Utilities|Text|ToText(String) (Utilities|String|Append (Utilities|String|ToString(Name) (Utilities|Struct|BreakStruct_Object (Variables|/Game/Blueprints/Objects/BP_Object.BP_Object_C|Getstructure (Variables|Construction|GetobjectConstruction)))) " déposé(e) !")) true 2.0)
  (Collision|SetActorEnableCollision (Variables|Construction|GetobjectConstruction) true)
  (Variables|Construction|SetisConstruction false)
  (Variables|Construction|SetobjectConstruction 0))

(fn Mourir
  (Variables|Constantes|SetisMort true)
  (Input|DisableInput (Game|GetPlayerController 0)))

(fn GestionSoif
  (params (value :type Float%20%28single-precision%29))
  (bind _structout (Utilities|Struct|SetmembersinStruct_HeroConstantes (Variables|Constantes|Getconstantes) (Math|Float|Clamp(Float) (+ (.soif (Utilities|Struct|BreakStruct_HeroConstantes (Variables|Constantes|Getconstantes))) value) 0.0 (.soifMax (Utilities|Struct|BreakStruct_HeroConstantes (Variables|Constantes|Getconstantes))))))
  (Variables|Constantes|Setconstantes _structout))

(fn GestionFaim
  (params (value :type Float%20%28single-precision%29))
  (bind _structout (Utilities|Struct|SetmembersinStruct_HeroConstantes (Variables|Constantes|Getconstantes) (Math|Float|Clamp(Float) (+ (.faim (Utilities|Struct|BreakStruct_HeroConstantes (Variables|Constantes|Getconstantes))) value) 0.0 (.faimMax (Utilities|Struct|BreakStruct_HeroConstantes (Variables|Constantes|Getconstantes))))))
  (Variables|Constantes|Setconstantes _structout))