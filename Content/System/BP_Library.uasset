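; BP_Library is a function library of global shortcuts to the custom game mode, player hero and player controller.
; Each getter casts the engine's game mode, first player character or first player controller to its project class, with the hero also checked for validity.
; Print String Information builds on the controller getter to send text, fade and duration to the main UI's information text.
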(fn CastGameModeCustom
  (bind _asgame_mode_custom (Utilities|Casting|CastToGameModeCustom (Game|GetGameMode (LocalVariables|Get__WorldContext))))
  (return _asgame_mode_custom))

(fn CastHeroPlayer
  (bind _asbp_hero (Utilities|Casting|CastToBP_Hero (Game|GetPlayerCharacter 0)))
  (Utilities|IsValid _asbp_hero
    (:Is%20Valid
      (return _asbp_hero))))

(fn CastPlayerControllerCustom
  (bind _asplayer_controller_custom (Utilities|Casting|CastToPlayerControllerCustom (Game|GetPlayerController 0)))
  (return _asplayer_controller_custom))

(fn PrintStringInformation
  (params (text :type Text) (fade :type Boolean) (duration :type Float%20%28single-precision%29))
  (Default|UpdateInformationsText (Variables|/Game/System/PlayerControllerCustom.PlayerControllerCustom_C|GetmainUI (CallFunction|CastPlayerControllerCustom (LocalVariables|Get__WorldContext))) text fade duration))