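; BP_Object is a pickup item that outlines itself via custom depth and shows a name widget while the player overlaps its box.
; On interaction, it adds its class to the hero's inventory, plays a sound and destroys itself, even if the inventory is full.
; Stackable items increment a matching entry; otherwise the first empty slot past a reserved index range is used, with on-screen feedback.
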(event OnComponentBeginOverlap(Box)
  (params (OverlappedComponent :type Primitive%20Component%20Object%20Reference) (OtherActor :type Actor%20Object%20Reference) (OtherComp :type Primitive%20Component%20Object%20Reference) (OtherBodyIndex :type Integer) (bFromSweep :type Boolean) (SweepResult :type Hit%20Result%20Structure%20%28by%20ref%29))
  ;[1 1 1] Begin Overlap : Affiche l'objet et son nom
  (if (== OtherActor (Game|GetPlayerCharacter 0))
    (Rendering|SetRenderCustomDepth (Variables|Default|GetMesh) true)
    (Rendering|SetVisibility (Variables|Default|GetWidgetNom) true false)
    (Utilities|FlowControl|DoOnce false
      (:Completed
        (bind _asbp_object_tooltip (Utilities|Casting|CastToBP_Object_Tooltip (UserInterface|GetUserWidgetObject (Variables|Default|GetWidgetNom))))
        (Default|SetNameText _asbp_object_tooltip (.nom (Utilities|Struct|BreakStruct_Object (Variables|Default|Getstructure))))))))

(event OnComponentEndOverlap(Box)
  (params (OverlappedComponent :type Primitive%20Component%20Object%20Reference) (OtherActor :type Actor%20Object%20Reference) (OtherComp :type Primitive%20Component%20Object%20Reference) (OtherBodyIndex :type Integer))
  ;[1 1 1] End Overlap : Cache l'objet et le outline
  (if (== OtherActor (Game|GetPlayerCharacter 0))
    (Rendering|SetRenderCustomDepth (Variables|Default|GetMesh) false)
    (Rendering|SetVisibility (Variables|Default|GetWidgetNom) false false)))

(event EventIInteraction
  ;[1 1 1] Interaction avec l'objet
  (Hero|AddObjectInventaire (Utilities|GetClass self) (Variables|Default|Getstructure)) ; Ajoute élément à l'inventaire
  (Audio|PlaySoundatLocation "/Game/Sounds/Cue_Get_Item.Cue_Get_Item" (Transformation|GetActorLocation self) "0, 0, 0" 1.0 1.0 0.0 0 0 0)
  (Actor|DestroyActor) ; Supprime l'élément du jeu
)

(fn ConstructionScript)

(fn AddObjectInventaire
  (params (object :type BP%20Object%20Class%20Reference) (objectStructur :type Struct%20Object%20Structure))
  (bind _asbp_hero (CallFunction|CastHeroPlayer))
  (bind _asbp_hero_2 (CallFunction|CastHeroPlayer))
  (bind _inventaire (Variables|/Game/Hero/BP_Hero.BP_Hero_C|Getinventaire _asbp_hero))
  (bind _inventaire_2 (Variables|/Game/Hero/BP_Hero.BP_Hero_C|Getinventaire _asbp_hero_2))
  (LocalVariables|SetobjectLocal object)
  ;[1 1 1] Test si l'objet est stackable
  (if (Utilities|Struct|BreakStruct_Object objectStructur)
    ;[1 1 1] Si l'objet stackable est trouvé dans l'inventaire on incrémente sa quantité
    (bind _index (Utilities|FlowControl|ForLoopwithBreak 9 (- (Utilities|Array|Length _inventaire_2) 1))
      (:LoopBody
        (bind _output_get (LocalVariables|SetindexArrayStackable _index))
        (if (Utilities|IsValidClass (.objectClass (Utilities|Struct|BreakStruct_InventaireHero (Utilities|Array|Get(acopy) _inventaire_2 _output_get))))
          (if (== (LocalVariables|GetobjectLocal) (.objectClass (Utilities|Struct|BreakStruct_InventaireHero (Utilities|Array|Get(acopy) _inventaire_2 _output_get))))
            (bind _structout (Utilities|Struct|SetmembersinStruct_InventaireHero (Utilities|Struct|MakeStruct_InventaireHero (.objectClass (Utilities|Struct|BreakStruct_InventaireHero (Utilities|Array|Get(acopy) _inventaire_2 _output_get))) (+ (.quantity (Utilities|Struct|BreakStruct_InventaireHero (Utilities|Array|Get(acopy) _inventaire_2 _output_get))) 1))))
            (Utilities|Array|SetArrayElem _inventaire_2 (LocalVariables|GetindexArrayStackable) _structout)
            (LocalVariables|SetisStackableFind true)
            ;[1 1 1] Message informant quel objet à été ramassé
            (CallFunction|PrintStringInformation (Utilities|Text|ToText(String) (Utilities|String|Append "+1 " (Utilities|String|ToString(Name) (.nom (Utilities|Struct|BreakStruct_Object (Utilities|GetClassDefaults (.objectClass (Utilities|Struct|BreakStruct_InventaireHero _structout)))))))) true 2.0))))
      (:Completed
        ;[1 1 1] Si l'object est stackable mais pas encore dans l'inventaire
        (if (not (LocalVariables|GetisStackableFind))
          ;[1 1 1] Si object pas stackable, on cherche un slot vide
          (bind _index_2 (Utilities|FlowControl|ForLoopwithBreak 9 (- (Utilities|Array|Length _inventaire) 1) :!label _label)
            (:LoopBody
              (bind _output_get_2 (LocalVariables|SetindexArray _index_2))
              (if (not (Utilities|IsValidClass (Utilities|Struct|BreakStruct_InventaireHero (Utilities|Array|Get(acopy) _inventaire _output_get_2))))
                (LocalVariables|SetisFind true)
                (goto _label Break)))
            (:Completed
              (if (LocalVariables|GetisFind)
                ;[1 1 1] Si un slot vide est trouvé, on le modifie pour ajouter l'object ramassé
                (bind _structout_2 (Utilities|Struct|SetmembersinStruct_InventaireHero (Utilities|Struct|MakeStruct_InventaireHero (LocalVariables|GetobjectLocal) 1)))
                (Utilities|Array|SetArrayElem _inventaire (LocalVariables|GetindexArray) _structout_2)
                ;[1 1 1] Message informant quel objet à été ramassé
                (CallFunction|PrintStringInformation (Utilities|Text|ToText(String) (Utilities|String|Append "+" (Utilities|String|ToString(Integer) (.quantity (Utilities|Struct|BreakStruct_InventaireHero _structout_2))) " " (Utilities|String|ToString(Name) (.nom (Utilities|Struct|BreakStruct_Object (Utilities|GetClassDefaults (.objectClass (Utilities|Struct|BreakStruct_InventaireHero _structout_2)))))))) true 2.0)
                (else
                  ;[1 1 1] Si l'inventaire est plein
                  (CallFunction|PrintStringInformation "Inventaire plein" true 2.0))))))))
    (else
      (goto _label))))