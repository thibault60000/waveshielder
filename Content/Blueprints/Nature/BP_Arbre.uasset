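; Choppable tree actor that drops resources when its health runs out.
; Player overlap toggles the custom-depth highlight and a nature tooltip widget showing name and health.
; GestionVie adds a health delta and, if the tooltip is valid, triggers delayed bar and sound feedback, destroying at zero.
; Destruction scatters physics-toggled pickups at random reachable points, spawns a stump, and hands respawn to the game mode.
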(event OnComponentBeginOverlap(Box)
  (params (OverlappedComponent :type Primitive%20Component%20Object%20Reference) (OtherActor :type Actor%20Object%20Reference) (OtherComp :type Primitive%20Component%20Object%20Reference) (OtherBodyIndex :type Integer) (bFromSweep :type Boolean) (SweepResult :type Hit%20Result%20Structure%20%28by%20ref%29))
  ;[1 1 1] En entrant dans la zone de l'arbre
  (if (== OtherActor (Game|GetPlayerCharacter 0))
    (Rendering|SetRenderCustomDepth (Variables|Default|GetMeshArbre) true)
    (Rendering|SetVisibility (Variables|Default|GetWidget) true false)
    (Utilities|FlowControl|DoOnce false
      (:Completed
        (bind _asbp_nature_tooltip (Utilities|Casting|CastToBP_Nature_Tooltip (UserInterface|GetUserWidgetObject (Variables|Default|GetWidget))))
        (bind _output_get (Variables|Default|SettooltipNature _asbp_nature_tooltip))
        (Default|SetColors _output_get (Utilities|Struct|MakeLinearColor 0.026532 0.541667 0.0 1.0))
        (Default|SetNameText _output_get (Utilities|Struct|BreakStruct_Arbre (Variables|Default|GetstructureArbre)))))))

(event OnComponentEndOverlap(Box)
  (params (OverlappedComponent :type Primitive%20Component%20Object%20Reference) (OtherActor :type Actor%20Object%20Reference) (OtherComp :type Primitive%20Component%20Object%20Reference) (OtherBodyIndex :type Integer))
  ;[1 1 1] En sortant de la zone de l'arbre
  (if (== OtherActor (Game|GetPlayerCharacter 0))
    (Rendering|SetRenderCustomDepth (Variables|Default|GetMeshArbre) false)
    (Rendering|SetVisibility (Variables|Default|GetWidget) false false)))

(event Custom|retirerVieArbre
  ;[1 1 1] Retirer de la vie après un delay
  (Utilities|FlowControl|Delay 0.5)
  (Default|SetProgressVie (Variables|Default|GettooltipNature) (Variables|Default|Getvie) (Variables|Default|GetvieMax))
  (Audio|PlaySoundatLocation "/Game/Sounds/Cue_Coup_Dans_Bois.Cue_Coup_Dans_Bois" (Transformation|GetActorLocation self) "0, 0, 0" 1.0 1.0 0.0 0 0 0))

(event Custom|destroyArbre
  (bind _returnvalue (Math|Random|RandomFloatinRange 0.0 3.6e+02))
  (bind _self self)
  (bind _structurearbre (Variables|Default|GetstructureArbre))
  (bind _spawnobjects (Utilities|Struct|BreakStruct_Arbre _structurearbre))
  (bind _returnvalue_2 (Transformation|GetActorTransform _self))
  (Utilities|FlowControl|Delay 0.5)
  ;[1 1 1] Spawn chaque ressource générée par la destruction de l'arbre
  (for _index (range 1 (Utilities|Struct|BreakStruct_Arbre (Variables|Default|GetstructureArbre)))
    (bind _returnvalue_3 (Game|SpawnActorfromClass _spawnobjects (Math|Transform|MakeTransform (+ (.RandomLocation (AI|Navigation|GetRandomReachablePointinRadius (.location (Transformation|GetActorTransform)) 3.5e+02 0 0)) "0.000000, 0,100.000000") (Math|Rotator|MakeRotator _returnvalue _returnvalue _returnvalue) "0.600000,0.600000,0.600000") "AdjustIfPossibleButAlwaysSpawn" 0 (Utilities|GetClassDefaults _spawnobjects) 0))
    (Default|PhysicsToggle _returnvalue_3))
  ;[1 1 1] Fait apparaitre un tronc et detruit l'acteur
  (bind _returnvalue_4 (Game|SpawnActorfromClass "/Game/Blueprints/Nature/BP_TroncArbre.BP_TroncArbre_C" (Math|Transform|MakeTransform (.location _returnvalue_2) (.rotation _returnvalue_2) "0.500000,0.500000,0.500000") "AdjustIfPossibleButAlwaysSpawn" 0 0))
  (Default|RespawnArbre (CallFunction|CastGameModeCustom) (Utilities|GetClass self) (Transformation|GetActorTransform self) _returnvalue_4 (Variables|Default|GettimeToRespawn))
  (Actor|DestroyActor))

(event EventBeginPlay)

(event Collision|EventActorBeginOverlap
  (params (OtherActor :type Actor%20Object%20Reference)))

(event EventTick
  (params (DeltaSeconds :type Float%20%28single-precision%29)))

(fn ConstructionScript)

(fn GestionVie
  (params (vieParam :type Float%20%28single-precision%29))
  ;[1 1 1] Retire la vie de l'arbre
  (bind _output_get (LocalVariables|SetvieARetirer vieParam))
  (bind _output_get_2 (Variables|Default|Setvie (+ (Variables|Default|Getvie) _output_get)))
  ;[1 1 1] Modifie le pourcentage sur la barre de vie
  (Utilities|IsValid (Variables|Default|GettooltipNature)
    (:Is%20Valid
      (CallFunction|RetirerVieArbre)
      ;[1 1 1] Détruit l'arbre si la vie est à 0
      (if (<= _output_get_2 0.0)
        (CallFunction|DetruireArbre)))))

(fn DetruireArbre
  ;[1 1 1] Détruit l'arbre (custom event avec Delay)
  (CallFunction|DestroyArbre))