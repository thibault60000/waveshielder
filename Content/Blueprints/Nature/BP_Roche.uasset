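; BP_Roche is a harvestable rock that drops resource actors when hit and breaks apart when its health runs out.
; Overlapping its box shows the player a custom-depth highlight and a widget with name and health bar.
; GestionVie applies health changes, triggering delayed sound and bar updates, then spawning one resource or calling destruction.
; Destruction scatters several physics-toggled resources on random reachable points, fractures the destructible mesh, then removes the actor.
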(event OnComponentBeginOverlap(Box)
  (params (OverlappedComponent :type Primitive%20Component%20Object%20Reference) (OtherActor :type Actor%20Object%20Reference) (OtherComp :type Primitive%20Component%20Object%20Reference) (OtherBodyIndex :type Integer) (bFromSweep :type Boolean) (SweepResult :type Hit%20Result%20Structure%20%28by%20ref%29))
  ;[1 1 1] En entrant dans la zone de l'arbre
  (if (== OtherActor (Game|GetPlayerCharacter 0))
    (Rendering|SetRenderCustomDepth (Variables|Default|GetDestructible) true)
    (Rendering|SetVisibility (Variables|Default|GetWidget) true false)
    (Utilities|FlowControl|DoOnce false
      (:Completed
        (bind _asbp_nature_tooltip (Utilities|Casting|CastToBP_Nature_Tooltip (UserInterface|GetUserWidgetObject (Variables|Default|GetWidget))))
        (bind _output_get (Variables|Default|SetnatureTooltip _asbp_nature_tooltip))
        (Default|SetNameText _output_get (Utilities|Struct|BreakStruct_Roche (Variables|Default|GetStructure)))))))

(event OnComponentEndOverlap(Box)
  (params (OverlappedComponent :type Primitive%20Component%20Object%20Reference) (OtherActor :type Actor%20Object%20Reference) (OtherComp :type Primitive%20Component%20Object%20Reference) (OtherBodyIndex :type Integer))
  ;[1 1 1] En sortant de la zone de l'arbre
  (if (== OtherActor (Game|GetPlayerCharacter 0))
    (Rendering|SetRenderCustomDepth (Variables|Default|GetDestructible) false)
    (Rendering|SetVisibility (Variables|Default|GetWidget) false false)))

(event Custom|RetirerVieRoche
  ;[1 1 1] Retirer de la vie après un delay
  (Utilities|FlowControl|Delay 0.5)
  (Default|SetProgressVie (Variables|Default|GetnatureTooltip) (Variables|Default|Getvie) (Variables|Default|GetvieMax))
  (Audio|PlaySoundatLocation "/Game/Sounds/Cue_Coup_Dans_Roche.Cue_Coup_Dans_Roche" (Transformation|GetActorLocation self) "0, 0, 0" 1.0 1.0 0.0 0 0 0))

(event Custom|DestroyRoche
  (bind _returnvalue (Math|Random|RandomFloatinRange 0.0 3.6e+02))
  (bind _destructible (Variables|Default|GetDestructible))
  (bind _structure (Variables|Default|GetStructure))
  (bind _spawnobjects (Utilities|Struct|BreakStruct_Roche _structure))
  (Utilities|FlowControl|Delay 0.5)
  ;[1 1 1] Spawn chaque ressource générée par la roche
  (for _index (range 1 (.quantitySpawnObjects (Utilities|Struct|BreakStruct_Roche (Variables|Default|GetStructure))))
    (bind _returnvalue_2 (Game|SpawnActorfromClass _spawnobjects (Math|Transform|MakeTransform (+ (.RandomLocation (AI|Navigation|GetRandomReachablePointinRadius (.location (Transformation|GetActorTransform)) 3.5e+02 0 0)) "0.000000, 0,80.000000") (Math|Rotator|MakeRotator _returnvalue _returnvalue _returnvalue) "1,1,1") "AdjustIfPossibleButAlwaysSpawn" 0 (Utilities|GetClassDefaults _spawnobjects) 0))
    (Default|PhysicsToggle _returnvalue_2))
  ;[1 1 1] Détruire "Destructible Mesh"
  (Class|DestructibleComponent|ApplyDamage _destructible 1e+01 (Transformation|GetWorldLocation _destructible) (Math|Vector|GetForwardVector _destructible) 0.0)
  (Rendering|SetRenderCustomDepth (Variables|Default|GetDestructible) false)
  (Rendering|SetVisibility (Variables|Default|GetWidget) false false)
  (Utilities|FlowControl|Delay 2.5)
  (Actor|DestroyActor)
  (CallFunction|PrintStringInformation (Utilities|Text|ToText(String) (Utilities|String|Append (Utilities|String|ToString(Name) (Utilities|Struct|BreakStruct_Roche (Variables|Default|GetStructure))) " détruit(e) !")) true 2.0))

(event Custom|SpawnElements
  (bind _returnvalue (Math|Random|RandomFloatinRange 0.0 3.6e+02))
  (bind _structure (Variables|Default|GetStructure))
  (bind _spawnobjects (Utilities|Struct|BreakStruct_Roche _structure))
  (Utilities|FlowControl|Delay 0.5)
  ;[1 1 1] Spawn éléments de la roche
  (bind _returnvalue_2 (Game|SpawnActorfromClass _spawnobjects (Math|Transform|MakeTransform (+ (.RandomLocation (AI|Navigation|GetRandomReachablePointinRadius (.location (Transformation|GetActorTransform)) 2e+02 0 0)) "0.000000, 0,80.000000") (Math|Rotator|MakeRotator _returnvalue _returnvalue _returnvalue) "1,1,1") "AdjustIfPossibleButAlwaysSpawn" 0 (Utilities|GetClassDefaults _spawnobjects) 0))
  (Utilities|IsValid _returnvalue_2
    (:Is%20Valid
      (Default|PhysicsToggle _returnvalue_2))))

(event EventBeginPlay)

(event Collision|EventActorBeginOverlap
  (params (OtherActor :type Actor%20Object%20Reference)))

(event EventTick
  (params (DeltaSeconds :type Float%20%28single-precision%29)))

(fn ConstructionScript)

(fn GestionVie
  (params (vieParam :type Float%20%28single-precision%29))
  (if (not (Variables|Default|GetisDestroy))
    ;[1 1 1] Retire la vie du rocher
    (bind _output_get (LocalVariables|SetvieARetirer vieParam))
    (bind _output_get_2 (Variables|Default|Setvie (+ (Variables|Default|Getvie) _output_get)))
    ;[1 1 1] Modifie le pourcentage sur la barre de vie
    (Utilities|IsValid (Variables|Default|GetWidget)
      (:Is%20Valid
        (CallFunction|RetirerVieRoche)
        ;[1 1 1] Détruit l'arbre si la vie est à 0
        (if (<= _output_get_2 0.0)
          (Variables|Default|SetisDestroy true)
          (CallFunction|DetruireRoche)
          (else
            ;[1 1 1] Sinon, spawn éléments
            (CallFunction|SpawnElements)))))))

(fn DetruireRoche
  ;[1 1 1] Détruire roche (custom event delay)
  (CallFunction|DestroyRoche))