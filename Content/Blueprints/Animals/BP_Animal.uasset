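; Animal character that wanders, eats, flees when hurt and drops loot on death.
; AIMoveTo loops through random reachable points with eating pauses; PrendreDommages triggers a faster flight, always at half health or below, otherwise randomly.
; GestionVie applies health changes, updates the tooltip, plays a cry and triggers death, which spawns briefly physics-simulated loot before destroying the actor.
; The player entering its box shows the tooltip widget and custom-depth highlight.
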(event OnComponentBeginOverlap(Box)
  (params (OverlappedComponent :type Primitive%20Component%20Object%20Reference) (OtherActor :type Actor%20Object%20Reference) (OtherComp :type Primitive%20Component%20Object%20Reference) (OtherBodyIndex :type Integer) (bFromSweep :type Boolean) (SweepResult :type Hit%20Result%20Structure%20%28by%20ref%29))
  ;[1 1 1] En entrant dans la zone de l'animal
  (if (== OtherActor (Game|GetPlayerCharacter 0))
    (Rendering|SetRenderCustomDepth (Variables|Character|GetMesh) true)
    (Rendering|SetVisibility (Variables|Default|GetWidget) true false)
    (Utilities|FlowControl|DoOnce false
      (:Completed
        (bind _asbp_animal_tooltip (Utilities|Casting|CastToBP_animal_tooltip (UserInterface|GetUserWidgetObject (Variables|Default|GetWidget))))
        (bind _output_get (Variables|Default|SettooltipAnimal _asbp_animal_tooltip))
        (Default|SetNameText _output_get (Utilities|Struct|BreakStruct_Animal (Variables|Default|GetstructureAnimal)))))))

(event OnComponentEndOverlap(Box)
  (params (OverlappedComponent :type Primitive%20Component%20Object%20Reference) (OtherActor :type Actor%20Object%20Reference) (OtherComp :type Primitive%20Component%20Object%20Reference) (OtherBodyIndex :type Integer))
  ;[1 1 1] En sortant de la zone de l'animal
  (if (== OtherActor (Game|GetPlayerCharacter 0))
    (Rendering|SetRenderCustomDepth (Variables|Character|GetMesh) false)
    (Rendering|SetVisibility (Variables|Default|GetWidget) false false)))

(event Custom|SeBalader
  ;[1 1 1] Se Balader
  (AI|AIMoveTo self (.RandomLocation (AI|Navigation|GetRandomReachablePointinRadius (Transformation|GetActorLocation self) 1e+03 0 0)) 0 5e+01 false
    (:OnSuccess
      (Variables|Default|SetisEating true)
      (Utilities|FlowControl|Delay 4.8)
      (Variables|Default|SetisEating false)
      (if (not (Variables|Default|GetisDied))
        (CallFunction|SeBalader)))))

(event Custom|RetirerVieAnimal
  ;[1 1 1] Retirer vie animal (widget + son)
  (Utilities|FlowControl|Delay 0.5)
  (Default|SetProgressVie (Variables|Default|GettooltipAnimal) (Variables|Default|Getvie) (Variables|Default|GetvieMax))
  (Audio|PlaySoundatLocation "/Game/Sounds/Cue_Faon_Cri.Cue_Faon_Cri" (Transformation|GetActorLocation self) "0, 0, 0" 1.0 1.0 0.0 0 0 0))

(event Custom|PrendreDommages
  ;[1 1 1] L'animal prend des dégats puis prend la fuite
  (Class|NavMovementComponent|StopActiveMovement (Variables|Character|GetCharacterMovement))
  (Utilities|FlowControl|Delay 0.2)
  (Variables|Default|SetisEating false)
  (Variables|Default|SetisDamaged true)
  (Utilities|FlowControl|Delay 0.5)
  (Variables|Default|SetisDamaged false)
  (if (<= (Variables|Default|Getvie) (/ (Variables|Default|GetvieMax) 2.0))
    (CallFunction|Fuite :!label _label)
    (elif (Math|Random|RandomBool)
      (goto _label)
      (else
        (CallFunction|SeBalader)))))

(event Custom|Fuite
  ;[1 1 1] Animal prend la fuite et se remet à se balader
  (Variables|/Script/Engine.CharacterMovementComponent|SetMaxWalkSpeed (Variables|Character|GetCharacterMovement) 4.8e+02)
  (AI|AIMoveTo self "0, 0, 0" 0 8e+01 false
    (:OnSuccess
      _)
    (:OnFail
      _))
  (Variables|/Script/Engine.CharacterMovementComponent|SetMaxWalkSpeed (Variables|Character|GetCharacterMovement) 1.4e+02)
  (CallFunction|SeBalader))

(event Custom|StopAnimalMort
  ;[1 1 1] Animation mort : désactiver tout
  (Utilities|FlowControl|Delay 0.2)
  (Utilities|FlowControl|Sequence
    (:then_0
      (Variables|Default|SetisEating false))
    (:then_1
      (Variables|Default|SetisDied true)
      (CallFunction|PrintStringInformation (Utilities|Text|ToText(String) (Utilities|String|Append "Vous avez tué : " (Utilities|String|ToString(Name) (.nom (Utilities|Struct|BreakStruct_Animal (Variables|Default|GetstructureAnimal)))))) true 2.5)
      (Pawn|Components|CharacterMovement|DisableMovement (Variables|Character|GetCharacterMovement))
      (AI|Navigation|StopMovement (AI|GetAIController self))
      (CallFunction|DisparitionAnimal))
    (:then_2
      (Variables|Default|SetisDamaged false))))

(event Custom|DisparitionAnimal
  (bind _returnvalue (Math|Random|RandomFloatinRange 0.0 3.6e+02))
  (bind _structureanimal (Variables|Default|GetstructureAnimal))
  (bind (_nom _dégat _loot) (Utilities|Struct|BreakStruct_Animal _structureanimal))
  ;[1 1 1] Fait spawn la viande
  (Utilities|FlowControl|Delay 4.0)
  (for _index (range 1 (.lootQuantity (Utilities|Struct|BreakStruct_Animal (Variables|Default|GetstructureAnimal))))
    (bind _returnvalue_2 (Game|SpawnActorfromClass _loot (Math|Transform|MakeTransform (+ (.RandomLocation (AI|Navigation|GetRandomReachablePointinRadius (.location (Transformation|GetActorTransform)) 2.5e+02 0 0)) "0.000000, 0,5.000000") (Math|Rotator|MakeRotator _returnvalue _returnvalue _returnvalue) "1,1,1") "AdjustIfPossibleButAlwaysSpawn" 0 (Utilities|GetClassDefaults _loot) 0))
    (Physics|SetSimulatePhysics (Variables|/Game/Blueprints/Objects/BP_Object.BP_Object_C|GetMesh _returnvalue_2) true)
    (Class|PrimitiveComponent|SetMassOverrideinKg (Variables|/Game/Blueprints/Objects/BP_Object.BP_Object_C|GetMesh _returnvalue_2) "None" 5e+02 true)
    (Utilities|FlowControl|Delay 3.0)
    (Physics|SetSimulatePhysics (Variables|/Game/Blueprints/Objects/BP_Object.BP_Object_C|GetMesh _returnvalue_2) false))
  (Actor|DestroyActor))

(event EventBeginPlay
  ;[1 1 1] Début de jeu : Lance la Balade
  (CallFunction|SeBalader))

(event Collision|EventActorBeginOverlap
  (params (OtherActor :type Actor%20Object%20Reference)))

(event EventTick
  (params (DeltaSeconds :type Float%20%28single-precision%29)))

(fn ConstructionScript)

(fn GestionVie
  (params (value :type Float%20%28single-precision%29))
  ;[1 1 1] Gestion de la vie, si 0 => tuer animal
  (bind _output_get (LocalVariables|SetvieARetirer value))
  (bind _output_get_2 (Variables|Default|Setvie (+ (Variables|Default|Getvie) _output_get)))
  (Utilities|IsValid (Variables|Default|GetWidget)
    (:Is%20Valid
      (CallFunction|RetirerVieAnimal)
      (if (<= _output_get_2 0.0)
        (CallFunction|StopAnimalMort)))))