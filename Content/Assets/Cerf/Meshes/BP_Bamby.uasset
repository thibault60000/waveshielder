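; BP_Bamby is a wandering deer pawn that reveals an animal tooltip when the player approaches.
; It loops AI moves to random reachable nearby points, setting IsEating during a pause after each successful arrival; failed moves do not restart the loop.
; Player overlap with its Box enables mesh custom depth and shows the Widget, filling its name once from StructureAnimal.
; No end-overlap handler hides either again.
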(event OnComponentBeginOverlap(Box)
  (params (OverlappedComponent :type Primitive%20Component%20Object%20Reference) (OtherActor :type Actor%20Object%20Reference) (OtherComp :type Primitive%20Component%20Object%20Reference) (OtherBodyIndex :type Integer) (bFromSweep :type Boolean) (SweepResult :type Hit%20Result%20Structure%20%28by%20ref%29))
  ;[1 1 1] En entrant dans la zone de l'animal
  (if (== OtherActor (Game|GetPlayerCharacter 0))
    (Rendering|SetRenderCustomDepth (Variables|Character|GetMesh) true)
    (Rendering|SetVisibility (Variables|Default|GetWidget) true false)
    (Utilities|FlowControl|DoOnce false
      (:Completed
        (bind _asbp_animal_tooltip (Utilities|Casting|CastToBP_animal_tooltip (UserInterface|GetUserWidgetObject (Variables|Default|GetWidget)))
          (:then
            (Development|PrintString "Hello")
            (Default|SetNameText _asbp_animal_tooltip (Utilities|Struct|BreakStruct_Animal (Variables|Default|GetstructureAnimal))))
          (:CastFailed
            (Development|PrintString "azeaz")))))))

(event Custom|SeBalader
  (AI|AIMoveTo self (.RandomLocation (AI|Navigation|GetRandomReachablePointinRadius (Transformation|GetActorLocation self) 1e+03 0 0)) 0 5e+01 false
    (:OnSuccess
      (Variables|Default|SetisEating true)
      (Utilities|FlowControl|Delay 4.8)
      (Variables|Default|SetisEating false)
      (CallFunction|SeBalader))))

(event EventBeginPlay
  (CallFunction|SeBalader))

(event Collision|EventActorBeginOverlap
  (params (OtherActor :type Actor%20Object%20Reference)))

(event EventTick
  (params (DeltaSeconds :type Float%20%28single-precision%29)))

(fn ConstructionScript)